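; AI controller that runs a supplied behavior tree and feeds its blackboard with sight information about one target pawn.
; SetupAIC starts the tree and writes the Target and Origin keys, taking Origin from the controlled pawn's location.
; Sighting the target through PawnSensing sets CanSeeTarget and RecentlySeenTarget.
; A retriggerable delay of twice the sensing interval resets CanSeeTarget when sightings stop, while RecentlySeenTarget is not cleared here.
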(event `self.ReceiveBeginPlay`)

(event `Setup AIC`
  (params (BT :type "BehaviorTree Object Reference") (`PawnSensing target` :type "Pawn Object Reference"))
  (set `self.BT` BT)
  (set `self.PawnSensing target` `PawnSensing target`)
  (`self.RunBehaviorTree` (`self.BT`))
  (`/Game/Blueprints/BehaviorTree/BPL_MyAI.UpdateBBKey` self "Target" true (`self.PawnSensing target`) "NewEnumerator1")
  (`/Game/Blueprints/BehaviorTree/BPL_MyAI.UpdateBBKey` self "Origin" true (`self.PawnSensing target`) "NewEnumerator2" (`self.K2_GetActorLocation` (`self.K2_GetPawn`)))
  (set `self.IsUsingPawnSensing?` false))

(event `self.PawnSensing.OnSeePawn`
  (params (Pawn :type "Pawn Object Reference"))
  (if (not (`self.IsUsingPawnSensing?`))
    (if (== Pawn (`self.PawnSensing target`))
      (`|ExecutionSequence`
        (:`then_0`
          (`/Game/Blueprints/BehaviorTree/BPL_MyAI.UpdateBBKey` self "CanSeeTarget" true)
          (`KismetSystemLibrary.PrintString` "Can see")
          (`KismetSystemLibrary.RetriggerableDelay` (* (`PawnSensingComponent.SensingInterval` (`self.PawnSensing`)) 2.0))
          (`/Game/Blueprints/BehaviorTree/BPL_MyAI.UpdateBBKey` null "CanSeeTarget")
          (`KismetSystemLibrary.PrintString` "cant see"))
        (:`then_1`
          (`/Game/Blueprints/BehaviorTree/BPL_MyAI.UpdateBBKey` self "RecentlySeenTarget" true))))))

(fn `UserConstructionScript`)