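; A launcher component that fires a projectile toward a target location, meant to be called from a behavior tree task or the player.
; It spawns the configured projectile class at its own world transform, then sets the projectile movement component's velocity to the unit direction to the target times a speed variable.
; A successful launch plays an attenuated explosion sound and spawns an emitter at the origin; a missing movement component prints an error.
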(event `Launc Projectile at Location`
  (params (TargetLocation :type "Vector Structure"))
  (bind _returnvalue_location (`KismetMathLibrary.BreakTransform` (`self.K2_GetComponentToWorld`)))
  (bind _returnvalue_location_2 (`KismetMathLibrary.BreakTransform` (`self.K2_GetComponentToWorld`)))
  ;[1 1 1] Called from BTT or player
  (set `self.TargetLocation` TargetLocation)
  ;[1 1 1] Launch projectile
  (bind _returnvalue (`|SpawnActorFromClass` (`self.Proj Class`) (`self.K2_GetComponentToWorld`) "Undefined" "OverrideRootScale" null null))
  (bind _returnvalue_2 (`Actor.GetComponentByClass` _returnvalue "/Script/Engine.ProjectileMovementComponent"))
  (`/Engine/EditorBlueprintResources/StandardMacros.IsValid` _returnvalue_2
    (:`Is Valid`
      (set `self.ProjectileCompMovementRef` _returnvalue_2)
      ;[1 1 1] Velocity
      (set `MovementComponent.Velocity` (* (`KismetMathLibrary.GetDirectionUnitVector` _returnvalue_location (`self.TargetLocation`)) (`self.Speed`)) (`self.ProjectileCompMovementRef`))
      ;[1 1 1] Feedback
      (`GameplayStatics.SpawnSoundAtLocation` "/Game/StarterContent/Audio/Explosion01.Explosion01" _returnvalue_location_2 (struct) 1.0 1.0 0.0 "/Game/Blueprints/BehaviorTree/Projectiles/MySoundAttenuation.MySoundAttenuation" null)
      (`GameplayStatics.SpawnEmitterAtLocation` null _returnvalue_location_2))
    (:`Is Not Valid`
      (`KismetSystemLibrary.PrintString` "Not working!"))))