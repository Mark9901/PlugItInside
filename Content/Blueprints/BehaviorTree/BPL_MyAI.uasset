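; Blueprint function library of AI helpers for writing blackboard values and safely fetching actor components.
; UpdateBBKey switches on a key type to set a Bool, Actor, Vector or Float value on the AI controller's blackboard.
; GetComponentIFValid looks up a component by class and returns it with a validity flag, printing a debug string when it is missing.
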(fn `GetComponentIFValid`
  (params (Owner :type "Actor Object Reference") (ComponentClass :type "ActorComponent Class Reference"))
  (returns (ComponentRef :type "ActorComponent Object Reference") (`Valid?` :type Boolean))
  (bind _returnvalue (`Actor.GetComponentByClass` Owner ComponentClass))
  (`/Engine/EditorBlueprintResources/StandardMacros.IsValid` _returnvalue
    (:`Is Valid`
      (return _returnvalue true))
    (:`Is Not Valid`
      (`KismetSystemLibrary.PrintString` null (`KismetStringLibrary.Concat_StrStr` "" (`KismetSystemLibrary.GetDisplayName` _returnvalue) "" (`KismetSystemLibrary.GetDisplayName` Owner)))
      (return null false))))

(fn `UpdateBBKey`
  (params (AIController :type "AIController Object Reference") (KeyName :type Name) (BoolValue :type Boolean) (ObjectValue :type "Object Object Reference") (`Key Type` :type "/Game/Blueprints/BehaviorTree/KeyTypes Enum" :default "NewEnumerator0") (VectorValue :type "Vector Structure") (FloatValue :type "Float (single-precision)"))
  (bind _returnvalue (`AIBlueprintHelperLibrary.GetBlackboard` AIController))
  (bind _returnvalue_2 (`KismetSystemLibrary.MakeLiteralName` KeyName))
  (switch `/Game/Blueprints/BehaviorTree/KeyTypes` `Key Type`
    (:`NewEnumerator0`
      (`BlackboardComponent.SetValueAsBool` _returnvalue _returnvalue_2 BoolValue))
    (:`NewEnumerator1`
      (`BlackboardComponent.SetValueAsObject` _returnvalue _returnvalue_2 ObjectValue))
    (:`NewEnumerator2`
      (`BlackboardComponent.SetValueAsVector` _returnvalue _returnvalue_2 VectorValue))
    (:`NewEnumerator3`
      (`BlackboardComponent.SetValueAsFloat` _returnvalue _returnvalue_2 FloatValue))))