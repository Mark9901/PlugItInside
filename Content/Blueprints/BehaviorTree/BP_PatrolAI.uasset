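; Patrol AI pawn that runs a behavior tree through its My_AIC controller and can take damage.
; The construction script initializes its DamageableComponent at full health.
; On BeginPlay it passes the tree and the player pawn, as sensing target, to the controller.
; It then seeds a blackboard key with a random float derived from ProjectileLaunchingCooldown.
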(event `self.ReceiveBeginPlay`
  (bind _projectilelaunchingcooldown (`self.ProjectileLaunchingCooldown`))
  (bind _asmy_aic (cast `/Game/Blueprints/BehaviorTree/My_AIC` (`AIBlueprintHelperLibrary.GetAIController` self)))
  (`/Game/Blueprints/BehaviorTree/My_AIC.Setup AIC` _asmy_aic (`self.BT`) (`GameplayStatics.GetPlayerPawn` 0))
  (`/Game/Blueprints/BehaviorTree/BPL_MyAI.UpdateBBKey` (`AIBlueprintHelperLibrary.GetAIController` self) "None" false null "NewEnumerator3" (0.0 0.0 0.0) (`KismetMathLibrary.RandomFloatInRange` (/ _projectilelaunchingcooldown 2.0) (/ 0.5 _projectilelaunchingcooldown))))

(fn `UserConstructionScript`
  (`/Game/Blueprints/HealthSystem/DamageableComponent.Setup Damageable Component` (`self.DamageableComponent`) self (`self.Max Health`) (`self.Max Health`)))