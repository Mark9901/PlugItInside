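; Behavior tree task that teleports the AI-controlled pawn to a location stored in the blackboard.
; It spawns an emitter at the departure point, moves the pawn without sweeping, rotates it to look at the blackboard target actor, then spawns another emitter at the destination.
; The task completes immediately and always reports failure through FinishExecute(false).
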(event `self.ReceiveExecuteAI`
  (params (OwnerController :type "AIController Object Reference") (ControlledPawn :type "Pawn Object Reference"))
  (bind _returnvalue (`Actor.K2_GetActorLocation` ControlledPawn))
  (bind _returnvalue_2 (`BTFunctionLibrary.GetBlackboardValueAsVector` (`self.Teleport Location`)))
  (`GameplayStatics.SpawnEmitterAtLocation` null _returnvalue (struct))
  (`Actor.K2_SetActorLocation` ControlledPawn _returnvalue_2 false false)
  (`Actor.K2_SetActorRotation` ControlledPawn (`KismetMathLibrary.FindLookAtRotation` _returnvalue (`Actor.K2_GetActorLocation` (`BTFunctionLibrary.GetBlackboardValueAsActor` (`self.Target Key`)))) false)
  (`GameplayStatics.SpawnEmitterAtLocation` null _returnvalue_2)
  (`self.FinishExecute` false))