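; DamageableComponent is a health component that tracks damage for an owning actor and destroys it when health runs out.
; A setup event stores the owner, max health and current health.
; The damage event sets Health to the damage amount minus current Health, an inverted subtraction.
; At zero or below it prints a debug string and destroys the owner, otherwise it prints the hit amount.
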(event `Setup Damageable Component`
  (params (OwningActor :type "Actor Object Reference") (MaxHealth :type "Float (double-precision)") (Health :type "Float (double-precision)"))
  (set `self.OwningActor` OwningActor)
  (set `self.MaxHealth` MaxHealth)
  (set `self.Health` Health))

(event `Take Damage via Component`
  (params (DamageAmount :type "Float (double-precision)"))
  (set `self.Health` (- DamageAmount (`self.Health`)))
  (if (<= (`self.Health`) 0.0)
    (`KismetSystemLibrary.PrintString` "Hello")
    (`Actor.K2_DestroyActor` (`self.OwningActor`))
    (else
      (`KismetSystemLibrary.PrintString` (`KismetStringLibrary.Concat_StrStr` "Hit:" (`KismetStringLibrary.Conv_DoubleToString` DamageAmount))))))