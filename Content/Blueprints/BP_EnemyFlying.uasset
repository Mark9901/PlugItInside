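; BP_EnemyFlying is an enemy actor that spins its mesh on Tick and repeatedly fires at the player.
; BeginPlay starts a 0.2-second loop that aims ArrowShot at the player pawn and spawns BP_EnemyAttack there.
; A self-repeating event stores Arrow3's location as the target at random intervals and calls Moving.
; Movement looks unfinished: Alpha increments by zero, the Lerp is unused, and the mesh location is set to the origin.
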(event `self.ReceiveBeginPlay`
  (`self.Find next location`)
  (`self.ShootAtPlayer` :!label _label)
  (`KismetSystemLibrary.Delay` 0.2)
  (goto _label))

(event `Moving`
  (`KismetSystemLibrary.K2_SetTimerDelegate` (delegate `Moving`))
  (set `self.Alpha` (+ (`self.Alpha`) 0.0))
  (`SceneComponent.K2_SetWorldLocation` (`self.StaticMesh`) (0.0 0.0 0.0) false false))

(event `self.ReceiveTick`
  (params (DeltaSeconds :type "Float (single-precision)"))
  (`SceneComponent.K2_AddLocalRotation` (`self.StaticMesh`) (`KismetMathLibrary.MakeRotator` 0.0 0.0 (`self.delta rotation z yaw`)) false false))

(event `Find next location`
  (bind _array (`|MakeArray` (`self.Arrow3`)))
  (set `self.Location to move` (`SceneComponent.K2_GetComponentLocation` (`|GetArrayItem` _array (`KismetMathLibrary.RandomIntegerInRange` 0 (`KismetArrayLibrary.Array_LastIndex` _array)))))
  (`self.Moving`)
  (`KismetSystemLibrary.Delay` (`KismetMathLibrary.RandomFloatInRange` 2.0 4.0))
  (`self.Find next location`))

(event `ShootAtPlayer`
  (bind _arrowshot (`self.ArrowShot`))
  (`SceneComponent.K2_SetWorldRotation` _arrowshot (`KismetMathLibrary.FindLookAtRotation` (`SceneComponent.K2_GetComponentLocation` _arrowshot) (`SceneComponent.K2_GetComponentLocation` (`Actor.RootComponent` (`GameplayStatics.GetPlayerPawn` 0)))) false false)
  (`|SpawnActorFromClass` "/Game/Blueprints/BP_EnemyAttack.BP_EnemyAttack_C" (`SceneComponent.K2_GetComponentToWorld` (`self.ArrowShot`)) "Undefined" "OverrideRootScale" null null))

(fn `UserConstructionScript`)