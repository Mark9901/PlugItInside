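; AI controller that runs a supplied behavior tree and reports sightings of one target pawn to the blackboard.
; SetupAIC stores the tree and target, then seeds the Target and Origin keys, the latter from the controlled pawn's location.
; Seeing the target sets CanSeeTarget? and RecentlySeenTarget?; a retriggerable delay of twice the sensing interval clears only the former.
; This built-in PawnSensing handling is skipped when the pawn has a CustomPawnSensingComponent.
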(event `Setup AIC`
  (params (BT :type "BehaviorTree Object Reference") (PawnSensingTarget :type "Pawn Object Reference"))
  ;[1 1 1] Setup
  (set `self.BT` BT)
  (set `self.PawnSensingTarget` PawnSensingTarget)
  (`self.RunBehaviorTree` (`self.BT`))
  (`/Game/Blueprints/BT/MyAIFunctions.UpdateBBKey` self "Target" "NewEnumerator1" true (`self.PawnSensingTarget`))
  (`/Game/Blueprints/BT/MyAIFunctions.UpdateBBKey` self "Origin" "NewEnumerator2" true null (`self.K2_GetActorLocation` (`self.K2_GetPawn`)))
  (set `self.IsUsingCustomPawnSensing?` (`KismetSystemLibrary.IsValid` (`self.GetComponentByClass` (`self.K2_GetPawn` self) "/Game/Blueprints/BT/PawnSensing/CustomPawnSensingComponent.CustomPawnSensingComponent_C"))))

(event `self.PawnSensing.OnSeePawn`
  (params (Pawn :type "Pawn Object Reference"))
  (if (not (`self.IsUsingCustomPawnSensing?`))
    ;[1 1 1] Pawn sensing
    (if (== Pawn (`self.PawnSensingTarget`))
      (`|ExecutionSequence`
        (:`then_0`
          (`/Game/Blueprints/BT/MyAIFunctions.UpdateBBKey` self "CanSeeTarget?" "NewEnumerator0" true)
          (`KismetSystemLibrary.RetriggerableDelay` (* (`PawnSensingComponent.SensingInterval` (`self.PawnSensing`)) 2.0))
          (`/Game/Blueprints/BT/MyAIFunctions.UpdateBBKey` self "CanSeeTarget?"))
        (:`then_1`
          (`/Game/Blueprints/BT/MyAIFunctions.UpdateBBKey` self "RecentlySeenTarget?" "NewEnumerator0" true))))))

(fn `UserConstructionScript`)