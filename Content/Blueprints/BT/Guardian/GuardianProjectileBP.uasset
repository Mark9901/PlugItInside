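; Guardian projectile Blueprint that destroys a BP_FlyingPawn when its BlockAll component hits one.
; The hit event ignores other actors, calls Detonate, then destroys the pawn; the graph never destroys the projectile itself.
; Detonate uses a DoOnce to spawn a pixelated Niagara effect and an attenuated, low-pitched explosion sound at the component's location.
; A delayed effect spawn is left unconnected and never runs.
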(event `self.BlockAll.OnComponentHit`
  (params (HitComponent :type "PrimitiveComponent Object Reference") (OtherActor :type "Actor Object Reference") (OtherComp :type "PrimitiveComponent Object Reference") (NormalImpulse :type "Vector Structure") (Hit :type "HitResult Structure (by ref)"))
  (bind _asbp_flying_pawn (cast `/Game/Migrate/Blueprints/Player/BP_FlyingPawn` OtherActor))
  (`self.Detonate`)
  (`self.K2_DestroyActor` _asbp_flying_pawn))

(event `Detonate`
  (bind _returnvalue (`SceneComponent.K2_GetComponentLocation` (`self.BlockAll`)))
  (`/Engine/EditorBlueprintResources/StandardMacros.DoOnce` false
    (:`Completed`
      (`NiagaraFunctionLibrary.SpawnSystemAtLocation` "/Game/Migrate/Materials/Materials/NS_PIxelated.NS_PIxelated" _returnvalue)
      (`GameplayStatics.SpawnSoundAtLocation` "/Game/StarterContent/Audio/Explosion02.Explosion02" _returnvalue (struct) 2.0 0.4 0.0 "/Game/Blueprints/BT/Projectiles/MySoundAttention.MySoundAttention" null))))

(event `self.ReceiveTick`
  (params (DeltaSeconds :type "Float (single-precision)")))

(fn `UserConstructionScript`)