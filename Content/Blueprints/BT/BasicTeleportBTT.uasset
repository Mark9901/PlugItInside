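; Behavior tree task that teleports the controlled AI pawn to a blackboard location and turns it toward its target.
; It spawns an explosion particle at the old position, sets the pawn's location without sweeping, then rotates it to look at the blackboard target actor.
; A second explosion plays at the destination, and the task immediately finishes with success.
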(event `self.ReceiveExecuteAI`
  (params (OwnerController :type "AIController Object Reference") (ControlledPawn :type "Pawn Object Reference"))
  (bind _returnvalue (`Actor.K2_GetActorLocation` ControlledPawn))
  (bind _returnvalue_2 (`BTFunctionLibrary.GetBlackboardValueAsVector` (`self.TeleportLocation`)))
  (`GameplayStatics.SpawnEmitterAtLocation` "/Game/StarterContent/Particles/P_Explosion.P_Explosion" _returnvalue)
  (`Actor.K2_SetActorLocation` ControlledPawn _returnvalue_2 false false)
  (`Actor.K2_SetActorRotation` ControlledPawn (`KismetMathLibrary.FindLookAtRotation` _returnvalue (`Actor.K2_GetActorLocation` (`BTFunctionLibrary.GetBlackboardValueAsActor` (`self.TargetKey`)))) false)
  (`GameplayStatics.SpawnEmitterAtLocation` "/Game/StarterContent/Particles/P_Explosion.P_Explosion" _returnvalue_2)
  (`self.FinishExecute` true))