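; PatrollingAI is an AI-controlled pawn Blueprint that hands its behavior to a behavior tree run through a My_AIC controller.
; On BeginPlay it passes its behavior tree and player pawn 0, as the sensing target, to the controller's SetupAIC.
; It then seeds the Cooldown01 blackboard key with a random value between half and double ProjectileLaunchingCooldown, so the starting cooldown varies per instance.
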(event `self.ReceiveBeginPlay`
  (bind _projectilelaunchingcooldown (`self.ProjectileLaunchingCooldown`))
  (bind _asmy_aic (cast `/Game/Blueprints/BT/My_AIC` (`AIBlueprintHelperLibrary.GetAIController` self)))
  (`/Game/Blueprints/BT/My_AIC.Setup AIC` _asmy_aic (`self.BT`) (`GameplayStatics.GetPlayerPawn` 0))
  (`/Game/Blueprints/BT/MyAIFunctions.UpdateBBKey` (`AIBlueprintHelperLibrary.GetAIController` self) "Cooldown01" "NewEnumerator3" false null (0.0 0.0 0.0) (`KismetMathLibrary.RandomFloatInRange` (/ _projectilelaunchingcooldown 2.0) (/ _projectilelaunchingcooldown 0.5))))

(fn `UserConstructionScript`)