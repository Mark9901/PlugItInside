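; Enemy spawner actor that repeatedly spawns batches of a given enemy class on a timer.
; SpawnEnemies spawns the requested count at the supplied transform, waits SpawnDelay, then calls itself with the same class and count at the spawner's own transform, looping without an end condition.
; BeginPlay starts the loop with a count of zero and no class set, so that call spawns nothing.
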(event `self.ReceiveBeginPlay`
  (`self.SpawnEnemies` null))

(event `SpawnEnemies`
  (params (Enemy :type "Actor Class Reference") (SpawnTransform :type "Transform Structure") (`Number of enemies` :type Integer))
  (for _ (range `Number of enemies`)
    (`|SpawnActorFromClass` Enemy SpawnTransform "Undefined" "OverrideRootScale" null null))
  (`KismetSystemLibrary.Delay` (`self.Spawn delay`))
  (`self.SpawnEnemies` (`self.Enemy`) (`self.GetTransform`) (`self.Number Of Enemies`)))

(fn `UserConstructionScript`)